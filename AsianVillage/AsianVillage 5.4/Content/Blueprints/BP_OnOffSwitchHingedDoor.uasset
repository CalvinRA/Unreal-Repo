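; BP_OnOffSwitchHingedDoor is an interactable switch that turns a linked hinged door on and off.
; Each Interact event flips IsActive, plays a 2D button click and prints a debug Activate or Deactivate message.
; It writes the new state straight to the IsOn variable of the HingedDoor reference; any door motion lies outside this Blueprint.
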(event `self.Interact`
  (bind _hingeddoor (`self.HingedDoor`))
  (if (not (`self.IsActive`))
    (set `self.IsActive` true)
    (`KismetSystemLibrary.PrintString` "Activate")
    (`GameplayStatics.PlaySound2D` "/Engine/VREditor/Sounds/UI/Click_on_Button.Click_on_Button" 1.0 1.0 0.0 null null)
    (set `/Game/Blueprints/BP_HingedDoor.IsOn` true _hingeddoor)
    (else
      (set `self.IsActive` false)
      (`KismetSystemLibrary.PrintString` "Deactivate")
      (`GameplayStatics.PlaySound2D` "/Engine/VREditor/Sounds/UI/Click_on_Button.Click_on_Button" 1.0 1.0 0.0 null null)
      (set `/Game/Blueprints/BP_HingedDoor.IsOn` false _hingeddoor))))

(fn `UserConstructionScript`)