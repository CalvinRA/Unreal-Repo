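; BP_Turret_Standard is a turret that repeatedly fires BP_Projectile actors.
; Tick runs into a Delay of Interval, which acts as the fire timer and spawns one projectile each time it completes.
; Each projectile takes its location and rotation from ProjectileSpawnPoint and its uniform scale from ProjectileScale, then receives LifeSpan so it expires automatically.
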(event `self.ReceiveTick`
  (params (DeltaSeconds :type "Float (single-precision)"))
  (`KismetSystemLibrary.Delay` (`self.Interval`))
  (bind _returnvalue (`|SpawnActorFromClass` "/Game/Blueprints/BP_Projectile.BP_Projectile_C" (`KismetMathLibrary.MakeTransform` (.location (`SceneComponent.K2_GetComponentToWorld` (`self.Projectile_Spawn_Point`))) (.rotation (`SceneComponent.K2_GetComponentToWorld` (`self.Projectile_Spawn_Point`))) (`KismetMathLibrary.Conv_DoubleToVector` (`self.Projectile_Scale`))) "Undefined" "MultiplyWithRoot" null null))
  (`self.SetLifeSpan` _returnvalue (`self.Life_Span`)))

(fn `UserConstructionScript`)