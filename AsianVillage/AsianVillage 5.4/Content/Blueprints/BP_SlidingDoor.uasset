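; Sliding double door that opens when the third-person player character enters its trigger volume and closes when they leave.
; Overlap events on DoorTrigger play or reverse the DoorSilde timeline, but only while the IsOn flag is set.
; Each timeline update sets the relative transforms of both door panels from separate left and right location tracks, with the right panel rolled or turned 180 degrees.
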(event `self.DoorTrigger.OnComponentBeginOverlap`
  (params (OverlappedComponent :type "PrimitiveComponent Object Reference") (OtherActor :type "Actor Object Reference") (OtherComp :type "PrimitiveComponent Object Reference") (OtherBodyIndex :type Integer) (bFromSweep :type Boolean) (SweepResult :type "HitResult Structure (by ref)"))
  (cast `/Game/ThirdPerson/Blueprints/BP_ThirdPersonCharacter` OtherActor)
  (if (`self.IsOn`)
    (bind (_direction _doorsildeleft _doorslideright) (`Timeline|DoorSilde` :!label _label)
      (:`Update`
        (`|ExecutionSequence`
          (:`then_0`
            (`SceneComponent.K2_SetRelativeTransform` (`self.DoorLeft`) (`KismetMathLibrary.MakeTransform` _doorsildeleft) false false))
          (:`then_1`
            (`SceneComponent.K2_SetRelativeTransform` (`self.DoorRight`) (`KismetMathLibrary.MakeTransform` _doorslideright (struct :`Yaw` 180.0)) false false)))))))

(event `self.DoorTrigger.OnComponentEndOverlap`
  (params (OverlappedComponent :type "PrimitiveComponent Object Reference") (OtherActor :type "Actor Object Reference") (OtherComp :type "PrimitiveComponent Object Reference") (OtherBodyIndex :type Integer))
  (cast `/Game/ThirdPerson/Blueprints/BP_ThirdPersonCharacter` OtherActor)
  (if (`self.IsOn`)
    (goto _label :!via `Reverse`)))

(fn `UserConstructionScript`)