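; Switch actor that turns a weak jump pad on and off when interacted with.
; Each Interact call flips an IsActive flag, prints a debug message and plays a button click sound.
; It sets the referenced JumpPadWeak's Velocity to a fixed launch value when active and to zero when inactive.
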(event `/Game/Blueprints/BP_Interact.Interact`
  (bind _jumppadweak (`self.JumpPadWeak`))
  (if (not (`self.IsActive`))
    (set `self.IsActive` true)
    (`KismetSystemLibrary.PrintString` "Activate")
    (`GameplayStatics.PlaySound2D` "/Engine/VREditor/Sounds/UI/Click_on_Button.Click_on_Button" 1.0 1.0 0.0 null null)
    (set `/Game/Blueprints/BP_JumpPadWeak.Velocity` 100.0 _jumppadweak)
    (else
      (set `self.IsActive` false)
      (`KismetSystemLibrary.PrintString` "Deactivate")
      (`GameplayStatics.PlaySound2D` "/Engine/VREditor/Sounds/UI/Click_on_Button.Click_on_Button" 1.0 1.0 0.0 null null)
      (set `/Game/Blueprints/BP_JumpPadWeak.Velocity` 0.0 _jumppadweak))))

(fn `UserConstructionScript`)