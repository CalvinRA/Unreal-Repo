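; BP_Turret_Trigger is a turret that fires BP_Projectile actors while something overlaps its trigger area.
; Tick starts disabled, turns on at Tigger_Area begin overlap and off at any end overlap, without filtering the overlapping actor.
; A Delay on Tick paces shots by Interval, spawning each projectile at ProjectileSpawnPoint with configurable scale and lifespan.
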(event `self.ReceiveBeginPlay`
  (`self.SetActorTickEnabled` false))

(event `self.ReceiveTick`
  (params (DeltaSeconds :type "Float (single-precision)"))
  (`KismetSystemLibrary.Delay` (`self.Interval`))
  (bind _returnvalue (`|SpawnActorFromClass` "/Game/Blueprints/BP_Projectile.BP_Projectile_C" (`KismetMathLibrary.MakeTransform` (.location (`SceneComponent.K2_GetComponentToWorld` (`self.Projectile_Spawn_Point`))) (.rotation (`SceneComponent.K2_GetComponentToWorld` (`self.Projectile_Spawn_Point`))) (`KismetMathLibrary.Conv_DoubleToVector` (`self.Projectile_Scale`))) "Undefined" "MultiplyWithRoot" null null))
  (`self.SetLifeSpan` _returnvalue (`self.Life_Span`)))

(event `self.Tigger_Area.OnComponentBeginOverlap`
  (params (OverlappedComponent :type "PrimitiveComponent Object Reference") (OtherActor :type "Actor Object Reference") (OtherComp :type "PrimitiveComponent Object Reference") (OtherBodyIndex :type Integer) (bFromSweep :type Boolean) (SweepResult :type "HitResult Structure (by ref)"))
  (`self.SetActorTickEnabled` true))

(event `self.Tigger_Area.OnComponentEndOverlap`
  (params (OverlappedComponent :type "PrimitiveComponent Object Reference") (OtherActor :type "Actor Object Reference") (OtherComp :type "PrimitiveComponent Object Reference") (OtherBodyIndex :type Integer))
  (`self.SetActorTickEnabled` false))

(fn `UserConstructionScript`)